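; BP_MyCharacter is an FPS character Blueprint with Fire input and prototype hitscan damage logic.
; Pressing Fire resets the current shot damage to its base value and sets a Firing flag, which release clears.
; Two disconnected trace chains never run: a camera multi-trace subtracting wall absorption before printing damage on enemies, and a line trace printing per-bone damage from a map.
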(event Input|ActionEvents|InputActionFire
  (params (Key :type Key%20Structure :default "None"))
  (:Pressed
    (Variables|Default|SetCurrentsShootDamage (Variables|Default|GetDamageBP))
    (Variables|Default|SetFiring true))
  (:Released
    (Variables|Default|SetFiring false)))

(fn ConstructionScript)